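; Camera pawn for building rooms onto the spaceship, with mouse screen-edge scrolling.
; CraftMode starts a looping timer that traces under the cursor and uses the hit component's tag to pick a side.
; A DoOnce gate spawns one ghost room at the ship's opposite-named point, offset by the ghost's matching point, and destroys it when the trace misses.
; CraftRoom replaces the ghost with a real room, handling only the East selection.
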(event Custom|CraftMode
  (bind _returnvalue (Utilities|Time|SetTimerbyEvent (delegate Custom|ghostConstruct) 0.1 true))
  (Variables|Default|SetTimerCraftMode _returnvalue))

(event Custom|ghostConstruct
  (bind _returnvalue (Game|GetPlayerController 0))
  (bind (_worldlocation _worlddirection) (Game|Player|ConvertMouseLocationToWorldSpace _returnvalue))
  (bind (_outhit _returnvalue_2) (Collision|LineTraceByChannel _worldlocation (+ _worldlocation (* _worlddirection 5e+04)) "TraceTypeQuery3" false 0 "ForDuration"))
  (if _returnvalue_2
    (Utilities|FlowControl|DoOnce false :!label _label
      (:Completed
        (CallFunction|SelectLocationGhistCraft (Utilities|Array|Get(acopy) (Variables|/Script/Engine.ActorComponent|GetComponentTags (.HitComponent (Collision|BreakHitResult _outhit)))))))
    (else
      (Utilities|FlowControl|Sequence
        (:then_0
          (goto _label Reset))
        (:then_1
          (Utilities|IsValid (Variables|Default|GetTemp%20GhostCraft)
            (:Is%20Valid
              (Actor|DestroyActor (Variables|Default|GetTemp%20GhostCraft))
              (Variables|Default|SetTemp%20GhostCraft 0))))))))

(event Custom|CraftRoom
  (params (Selection :type Name))
  (switch name Selection
    (:East
      (Game|SpawnActorfromClass "/Game/BP/Actor/BP_RoomConstruct_Master.BP_RoomConstruct_Master_C" (Math|Transform|MakeTransform (Transformation|GetActorLocation (Variables|Default|GetTemp%20GhostCraft)) "0, 0, 0" "1.000000,1.000000,1.000000") "Undefined" 0 0)
      (Utilities|IsValid (Variables|Default|GetTemp%20GhostCraft)
        (:Is%20Valid
          (Actor|DestroyActor (Variables|Default|GetTemp%20GhostCraft))
          (Variables|Default|SetTemp%20GhostCraft 0))))))

(event EventBeginPlay
  (bind _outactors (Actor|GetAllActorsOfClass "/Game/BP/Actor/BP_Spaceship_Master.BP_Spaceship_Master_C"))
  (Variables|Default|SetSpaceship%20Ref (Utilities|Array|Get(acopy) _outactors)))

(event Input|MouseEvents|MouseX
  (params (AxisValue :type Float%20%28single-precision%29))
  (bind _returnvalue (Game|GetPlayerController 0))
  (bind _returnvalue_2 (Utilities|Time|GetWorldDeltaSeconds))
  (bind _returnvalue_3 (Viewport|GetViewportSize))
  (bind _scrollspeed (Variables|Default|GetScrollSpeed))
  (bind _locationx (Game|Player|GetMousePosition _returnvalue))
  (bind _returnvalue_4 (* _scrollspeed _returnvalue_2))
  (bind _returnvalue_5 (/ _locationx (.x _returnvalue_3)))
  (if (> _returnvalue_5 0.98)
    (Transformation|AddActorWorldOffset (Math|Vector|MakeVector 0.0 (* _returnvalue_4 -1.0) 0.0))
    (elif (< _returnvalue_5 0.02)
      (Transformation|AddActorWorldOffset (Math|Vector|MakeVector 0.0 _returnvalue_4 0.0)))))

(event Input|MouseEvents|MouseY
  (params (AxisValue :type Float%20%28single-precision%29))
  (bind _returnvalue (Game|GetPlayerController 0))
  (bind _returnvalue_2 (Viewport|GetViewportSize))
  (bind _returnvalue_3 (Utilities|Time|GetWorldDeltaSeconds))
  (bind _scrollspeed (Variables|Default|GetScrollSpeed))
  (bind _locationy (Game|Player|GetMousePosition _returnvalue))
  (bind _returnvalue_4 (* _scrollspeed _returnvalue_3))
  (bind _returnvalue_5 (/ _locationy (.y _returnvalue_2)))
  (if (> _returnvalue_5 0.98)
    (Transformation|AddActorWorldOffset (Math|Vector|MakeVector _returnvalue_4 0.0 0.0))
    (elif (< _returnvalue_5 0.2)
      (Transformation|AddActorWorldOffset (Math|Vector|MakeVector (* _returnvalue_4 -1.0) 0.0 0.0)))))

(fn ConstructionScript)

(fn SelectLocationGhistCraft
  (params (Selection :type Name))
  (switch name Selection
    (:North
      (|ChecklocationNorth))
    (:South
      (|ChecklocationSouth))
    (:East
      (|ChecklocationEast))
    (:West
      (|ChecklocationEast_4))))