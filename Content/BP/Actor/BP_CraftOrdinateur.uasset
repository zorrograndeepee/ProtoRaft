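; BP_CraftOrdinateur is an interactable crafting computer actor that puts the player into construction mode.
; On BeginPlay it caches the first BP_Spaceship_Master found in the level and the player's BP_ThirdPersonCharacter.
; Its Interraction event switches the view target to the spaceship, shows the mouse cursor and sets the character's BInConstructionMode flag.
; It has no exit logic of its own.
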(event EventInterraction
  (params (Character%20Ref :type BP%20Third%20Person%20Character%20Object%20Reference))
  (bind _returnvalue (Game|GetPlayerController 0))
  (Game|Player|SetViewTargetwithBlend _returnvalue (Variables|Default|GetSpaceship%20Ref) 0.0 "VTBlend_Linear" 0.0 false)
  (Variables|/Script/Engine.PlayerController|SetbShowMouseCursor _returnvalue true)
  (Variables|/Game/BP/Actor/BP_ThirdPersonCharacter.BP_ThirdPersonCharacter_C|SetB_In%20Construction%20mode (Variables|Default|GetAs%20BP%20Third%20Person%20Character%20REF) true))

(event EventBeginPlay
  (bind _outactors (Actor|GetAllActorsOfClass "/Game/BP/Actor/BP_Spaceship_Master.BP_Spaceship_Master_C"))
  (Variables|Default|SetSpaceship%20Ref (Utilities|Array|Get(acopy) _outactors))
  (bind _asbp_third_person_character (Utilities|Casting|CastToBP_ThirdPersonCharacter (Game|GetPlayerCharacter 0)))
  (Variables|Default|SetAs%20BP%20Third%20Person%20Character%20REF _asbp_third_person_character))

(fn ConstructionScript)