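; BP_CraftTable is a crafting table actor that unlocks a level 1 set of craftable items for the player while nearby.
; Entering its box unlocks the items through the character's InventoryManagerComponent; leaving toggles the crafting and inventory displays and locks them again.
; Interacting also unlocks the items and toggles both displays.
; A helper function reads DT_Crafting but returns only the first found row's unlock state and item.
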(event OnComponentBeginOverlap(Box)
  (params (OverlappedComponent :type Primitive%20Component%20Object%20Reference) (OtherActor :type Actor%20Object%20Reference) (OtherComp :type Primitive%20Component%20Object%20Reference) (OtherBodyIndex :type Integer) (bFromSweep :type Boolean) (SweepResult :type Hit%20Result%20Structure%20%28by%20ref%29))
  (Utilities|Casting|CastToBP_ThirdPersonCharacter OtherActor)
  (CallFunction|ProxiTableCraft))

(event OnComponentEndOverlap(Box)
  (params (OverlappedComponent :type Primitive%20Component%20Object%20Reference) (OtherActor :type Actor%20Object%20Reference) (OtherComp :type Primitive%20Component%20Object%20Reference) (OtherBodyIndex :type Integer))
  (Utilities|Casting|CastToBP_ThirdPersonCharacter OtherActor)
  (CallFunction|ProxicraftNone))

(event Custom|Lock%20craft
  (for _array_element (Variables|Default|GetEitems%20Unlock%20Lvl%201)
    (Default|LockItem (Variables|/Game/BP/Actor/BP_ThirdPersonCharacter.BP_ThirdPersonCharacter_C|GetInventory%20Manager%20Component (Variables|Default|GetRefBP%20Third%20Person%20Character)) _array_element)))

(event Custom|Proxi%20table%20craft
  (for _array_element (Variables|Default|GetEitems%20Unlock%20Lvl%201)
    (Default|UnlockItemCrafting (Variables|/Game/BP/Actor/BP_ThirdPersonCharacter.BP_ThirdPersonCharacter_C|GetInventory%20Manager%20Component (Variables|Default|GetRefBP%20Third%20Person%20Character)) _array_element)))

(event Custom|Proxicraft%20none
  (bind _refbp_third_person_character (Variables|Default|GetRefBP%20Third%20Person%20Character))
  (bind _inventory_manager_component (Variables|/Game/BP/Actor/BP_ThirdPersonCharacter.BP_ThirdPersonCharacter_C|GetInventory%20Manager%20Component _refbp_third_person_character))
  (Default|ToggleCraftingDisplayOpen _inventory_manager_component)
  (Default|ToggleInventoryOpen _inventory_manager_component)
  (CallFunction|LockCraft))

(event EventBeginPlay
  (bind _asbp_third_person_character (Utilities|Casting|CastToBP_ThirdPersonCharacter (Game|GetPlayerCharacter 0)))
  (Variables|Default|SetRefBP%20Third%20Person%20Character _asbp_third_person_character))

(event Collision|EventActorBeginOverlap
  (params (OtherActor :type Actor%20Object%20Reference)))

(event EventInterraction
  (params (Character%20Ref :type BP%20Third%20Person%20Character%20Object%20Reference))
  (bind _refbp_third_person_character (Variables|Default|GetRefBP%20Third%20Person%20Character))
  (bind _inventory_manager_component (Variables|/Game/BP/Actor/BP_ThirdPersonCharacter.BP_ThirdPersonCharacter_C|GetInventory%20Manager%20Component _refbp_third_person_character))
  (for _array_element (Variables|Default|GetEitems%20Unlock%20Lvl%201)
    (Default|UnlockItemCrafting _inventory_manager_component _array_element))
  (Development|PrintString "Hello")
  (Default|ToggleCraftingDisplayOpen _inventory_manager_component)
  (Default|ToggleInventoryOpen _inventory_manager_component))

(fn ConstructionScript)

(fn GetLock/UnlockItem
  (bind _outrownames (DataTable|GetDataTableRowNames "/Game/InventorySystem/Datatables/DT_Crafting.DT_Crafting"))
  (for _array_element _outrownames
    (bind _returnvalue (Utilities|GetDataTableRow "/Game/InventorySystem/Datatables/DT_Crafting.DT_Crafting" _array_element)
      (:then
        (return (.IsUnlocked (Utilities|Struct|BreakFCraftingStruct _returnvalue)) (.ItemToCraft (Utilities|Struct|BreakFCraftingStruct _returnvalue)))))))