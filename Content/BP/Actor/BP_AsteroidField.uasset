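; BP_AsteroidField is an actor that scatters asteroids in a spherical shell when play begins.
; A BeginPlay loop spawns BP_MasterAsteroid actors at random directions and distances around the world origin, not the field actor's location.
; Each gets a random rotation and uniform scale, tuned by count, distance and scale variables.
; An unconnected construction-script variant would add local-space mesh instances instead, but never runs.
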(event EventBeginPlay
  (for _index (range 0 (Variables|Default|GetTotalPods))
    (Game|SpawnActorfromClass "/Game/BP/Actor/BP_MasterAsteroid.BP_MasterAsteroid_C" (Math|Transform|MakeTransform (* (Math|Random|RandomUnitVector) (Math|Random|RandomFloatinRange (Variables|Default|GetMinDistance) (Variables|Default|GetMaxDistance))) (Math|Random|RandomRotator false) (Math|Conversions|ToVector(Float) (* (Math|Random|RandomFloatinRange (Variables|Default|GetMinScale) (Variables|Default|GetMaxScale)) (Variables|Default|GetScaleMultiplier)))) "Undefined" 0 0)))

(fn ConstructionScript)