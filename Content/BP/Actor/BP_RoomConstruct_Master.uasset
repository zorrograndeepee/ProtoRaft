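; BP_RoomConstruct_Master is an actor Blueprint, named as a master for room construction, that gathers a room's pieces into one list.
; Its Construction Script fills the Wall array with eight Cube elements and Sol (French for floor).
; Nothing in this file reads the array, and the event graph holds only disabled BeginPlay, overlap and Tick stubs.
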(event EventBeginPlay)

(event Collision|EventActorBeginOverlap
  (params (OtherActor :type Actor%20Object%20Reference)))

(event EventTick
  (params (DeltaSeconds :type Float%20%28single-precision%29)))

(fn ConstructionScript
  (Variables|Default|SetWall (Utilities|Array|MakeArray (Variables|Default|GetCube1) (Variables|Default|GetCube8) (Variables|Default|GetCube3) (Variables|Default|GetCube) (Variables|Default|GetCube7) (Variables|Default|GetCube2) (Variables|Default|GetSol) (Variables|Default|GetCube6) (Variables|Default|GetCube5))))