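; BP_Spaceship_Master is a spaceship actor that flies forward every tick through a self-replenishing asteroid field.
; It fills a Box volume with randomly placed, rotated and scaled asteroids, then a looping timer tops up the overlap count to a maximum.
; Asteroids receive a ship reference, and an exposed event can re-randomize their transforms within the Box.
; Asteroids touching the ship's collision are destroyed; Cube interaction only prints a test message.
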(event OnComponentBeginOverlap(CollisionSpaceship)
  (params (OverlappedComponent :type Primitive%20Component%20Object%20Reference) (OtherActor :type Actor%20Object%20Reference) (OtherComp :type Primitive%20Component%20Object%20Reference) (OtherBodyIndex :type Integer) (bFromSweep :type Boolean) (SweepResult :type Hit%20Result%20Structure%20%28by%20ref%29))
  ;[1 1 1] destroy asterois in spaceship
  (bind _asbp_master_asteroid (Utilities|Casting|CastToBP_MasterAsteroid OtherActor))
  (Actor|DestroyActor _asbp_master_asteroid))

(event Custom|Spawn%20astoroid
  (bind _box (Variables|Default|GetBox))
  (bind (_origin _boxextent) (Collision|GetComponentBounds _box))
  (bind _returnvalue (Game|SpawnActorfromClass "/Game/BP/Actor/BP_MasterAsteroid.BP_MasterAsteroid_C" (Math|Transform|MakeTransform (Math|Random|RandomPointinBoundingBox _origin _boxextent) (Math|Random|RandomRotator false) (Math|Conversions|ToVector(Float) (* (Math|Random|RandomFloatinRange (Variables|Default|GetMinScale) (Variables|Default|GetMaxScale)) (Variables|Default|GetScaleMultiplier)))) "Undefined" 0 0))
  (Variables|/Game/BP/Actor/BP_MasterAsteroid.BP_MasterAsteroid_C|SetRef%20Spaceship _returnvalue self))

(event Custom|Check%20if%20asteroid%20is%20in%20box%20spaceship
  (if (< (Utilities|Array|Length (Collision|GetOverlappingActors (Variables|Default|GetBox) "/Game/BP/Actor/BP_MasterAsteroid.BP_MasterAsteroid_C" :!class /Script/Engine.PrimitiveComponent)) (Variables|Default|GetMaxAsteroidFrontOfTheSpaceship))
    (CallFunction|SpawnAstoroid)))

(event Custom|Start%20spawn%20asteroid
  (bind _box (Variables|Default|GetBox))
  (bind (_origin _boxextent) (Collision|GetComponentBounds _box))
  (for _index (range 0 (Variables|Default|GetMaxAsteroidFrontOfTheSpaceship))
    (bind _returnvalue (Game|SpawnActorfromClass "/Game/BP/Actor/BP_MasterAsteroid.BP_MasterAsteroid_C" (Math|Transform|MakeTransform (Math|Random|RandomPointinBoundingBox _origin _boxextent) (Math|Random|RandomRotator false) (Math|Conversions|ToVector(Float) (* (Math|Random|RandomFloatinRange (Variables|Default|GetMinScale) (Variables|Default|GetMaxScale)) (Variables|Default|GetScaleMultiplier)))) "Undefined" 0 0))
    (Variables|/Game/BP/Actor/BP_MasterAsteroid.BP_MasterAsteroid_C|SetRef%20Spaceship _returnvalue self))
  (Utilities|Time|SetTimerbyEvent (delegate Custom|Check%20if%20asteroid%20is%20in%20box%20spaceship) 0.1 true))

(event Custom|Spaceship%20move
  (Transformation|AddActorWorldOffset (* (Math|Vector|GetForwardVector (Transformation|GetActorRotation)) (Variables|Default|GetSpeed%20of%20the%20spaceship))))

(event Custom|Set%20location%20asteroid
  (params (Ref%20Asteroid :type BP%20Master%20Asteroid%20Object%20Reference))
  (bind _box (Variables|Default|GetBox))
  (bind (_origin _boxextent) (Collision|GetComponentBounds _box))
  (Transformation|SetActorTransform Ref%20Asteroid (Math|Transform|MakeTransform (Math|Random|RandomPointinBoundingBox _origin _boxextent) (Math|Random|RandomRotator false) (Math|Conversions|ToVector(Float) (* (Math|Random|RandomFloatinRange (Variables|Default|GetMinScale) (Variables|Default|GetMaxScale)) (Variables|Default|GetScaleMultiplier)))) false true))

(event EventTick
  (params (DeltaSeconds :type Float%20%28single-precision%29))
  (CallFunction|SpaceshipMove))

(event EventBeginPlay
  (CallFunction|StartSpawnAsteroid))

(event EventInterraction
  (params (Character%20Ref :type BP%20Third%20Person%20Character%20Object%20Reference) (Component :type Actor%20Component%20Object%20Reference))
  (Utilities|IsValid Component
    (:Is%20Valid
      (if (== Component (Variables|Default|GetCube))
        (Development|PrintString "Hello")))))

(fn ConstructionScript)